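; BP_EagleGlitchy is a moving hazard that kills the glitchy sprite character on contact.
; Its construction script gives an InterpToMovement component two relative control points, the origin and MovePosition, with CustomDistance used as the travel duration.
; On actor overlap, it casts the other actor to BP_SpirteCharacterGLITCHY and sets its DeadG flag, leaving any death handling to that character.
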(event EventBeginPlay)

(event Collision|EventActorBeginOverlap
  (params (OtherActor :type Actor%20Object%20Reference))
  (bind _asbp_spirte_character_glitchy (Utilities|Casting|CastToBP_SpirteCharacterGLITCHY OtherActor))
  (Variables|/Game/Blueprints/BP_SpirteCharacterGLITCHY.BP_SpirteCharacterGLITCHY_C|SetdeadG _asbp_spirte_character_glitchy true))

(fn ConstructionScript
  (Class|InterptoMovementComponent|AddControlPointPosition (Variables|Default|GetInterpToMovement) "0, 0, 0" true)
  (Class|InterptoMovementComponent|AddControlPointPosition (Variables|Default|GetInterpToMovement) (Variables|Default|GetmovePosition) true)
  (Variables|/Script/Engine.InterpToMovementComponent|SetDuration (Variables|Default|GetInterpToMovement) (Variables|Default|GetcustomDistance)))