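; BP_MovingPlatformSmall is a small moving platform drawn with a Paper2D tile map.
; The construction script gives its InterpToMovement component two relative control points, the origin and MovePosition, and sets the movement Duration from CustomDistance.
; On BeginPlay it applies the PaperTile variable as the tile map, and Tick does nothing.
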(event EventBeginPlay
  (Class|PaperTileMapComponent|SetTileMap (Variables|Default|GetPaperTileMap) (Variables|Default|GetpaperTile)))

(event EventTick
  (params (DeltaSeconds :type Float%20%28single-precision%29)))

(fn ConstructionScript
  (Class|InterptoMovementComponent|AddControlPointPosition (Variables|Default|GetInterpToMovement) "0, 0, 0" true)
  (Class|InterptoMovementComponent|AddControlPointPosition (Variables|Default|GetInterpToMovement) (Variables|Default|GetmovePosition) true)
  (Variables|/Script/Engine.InterpToMovementComponent|SetDuration (Variables|Default|GetInterpToMovement) (Variables|Default|GetcustomDistance)))