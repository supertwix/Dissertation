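; BP_Eagle is a moving hazard that kills the player's sprite character on contact.
; The construction script gives InterpToMovement a relative path from the actor's origin to MovePosition, using CustomDistance as the travel duration despite its name.
; On actor overlap, it casts the other actor to BP_SpirteCharacter and sets its Dead flag directly.
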(event EventBeginPlay)

(event Collision|EventActorBeginOverlap
  (params (OtherActor :type Actor%20Object%20Reference))
  (bind _asbp_spirte_character (Utilities|Casting|CastToBP_SpirteCharacter OtherActor))
  (Variables|/Game/Blueprints/BP_SpirteCharacter.BP_SpirteCharacter_C|Setdead _asbp_spirte_character true))

(fn ConstructionScript
  (Class|InterptoMovementComponent|AddControlPointPosition (Variables|Default|GetInterpToMovement) "0, 0, 0" true)
  (Class|InterptoMovementComponent|AddControlPointPosition (Variables|Default|GetInterpToMovement) (Variables|Default|GetmovePosition) true)
  (Variables|/Script/Engine.InterpToMovementComponent|SetDuration (Variables|Default|GetInterpToMovement) (Variables|Default|GetcustomDistance)))